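; BP_Explosion is a timed explosion actor that plays a visual blast and affects actors within its Radius.
; After a delay, a timeline scales the sphere, dithers its dynamic material and drives the point light, then destroys the actor.
; On detonation it also shakes cameras, fires a radial impulse, sends ExplosionHitMessage to overlapped actors and destroys those listed in DestroyOnExplode, which the overlap ignores.
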(event `self.ReceiveBeginPlay`
  (`|ExecutionSequence`
    (:`then_0`
      (if (== (`self.timeBeforeExplosion`) 0.0)
        (set `self.timeBeforeExplosion` 0.01)))
    (:`then_1`
      (bind _returnvalue (`PrimitiveComponent.CreateDynamicMaterialInstance` (`self.Sphere`) 0 "/Game/Materials/FX/MI_Explosion.MI_Explosion" "None"))
      (bind _output_get (set `self.mat` _returnvalue))
      (`PrimitiveComponent.SetMaterial` (`self.Sphere`) 0 _output_get)
      (set `RadialForceComponent.Radius` (`self.radius`) (`self.RadialForce`))
      (`KismetSystemLibrary.K2_SetTimerDelegate` (delegate `Explode`) (`self.timeBeforeExplosion`)))))

(event `Explode`
  (`|ExecutionSequence`
    (:`then_0`
      (bind (_direction _scale _dither _light_intensity) (`Timeline|ExplosionTL`)
        (:`Update`
          (bind _returnvalue (* _scale (/ (`self.radius`) 120.0)))
          (`SceneComponent.SetRelativeScale3D` (`self.Sphere`) (`KismetMathLibrary.MakeVector` _returnvalue _returnvalue _returnvalue))
          (`MaterialInstanceDynamic.SetScalarParameterValue` (`self.mat`) "Dither" _dither)
          (`LightComponent.SetIntensity` (`self.PointLight`) (* _light_intensity 3333.333333 (`self.radius`))))
        (:`Finished`
          (`self.K2_DestroyActor`))))
    (:`then_1`
      (`GameplayStatics.PlayWorldCameraShake` "/Game/FX/CS_Explosion.CS_Explosion_C" (`self.K2_GetActorLocation`) 0.0 4000.0 1.0 true)
      (`RadialForceComponent.FireImpulse` (`self.RadialForce`))
      (bind _outactors (`KismetSystemLibrary.SphereOverlapActors` (`self.K2_GetActorLocation`) (`self.radius`) (`|MakeArray` "ObjectTypeQuery1" "ObjectTypeQuery2" "ObjectTypeQuery6" "ObjectTypeQuery4" :!type "EObjectTypeQuery Enum") null (`self.destroyOnExplode`)))
      (for _array_element _outactors
        (message `/Game/BP/BPI/BPI_Explosion.explosionHit` _array_element)))
    (:`then_2`
      (for _array_element_2 (`self.destroyOnExplode`)
        (`/Engine/EditorBlueprintResources/StandardMacros.IsValid` _array_element_2
          (:`Is Valid`
            (`self.K2_DestroyActor` _array_element_2)))))))

(fn `UserConstructionScript`)